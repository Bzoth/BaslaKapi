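; BP_LogoPuzzle is a rotation puzzle with three sphere components that are each turned toward a target orientation.
; Puzzleer rolls the passed component 60 degrees through MoveComponentTo, using CanTurn to block overlapping turns, then calls CheckForWin.
; CheckForWin compares each sphere to its target within a tolerance, swaps its material to show correctness, and counts matches.
; When all three match, every sphere receives a solved material.
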(event `/Game/Blueprints/BPI_Puzzler.Puzzleer`
  (params (NewParam :type "SceneComponent Object Reference"))
  (bind (_relativerotation_roll _relativerotation_pitch _relativerotation_yaw) (`KismetMathLibrary.BreakRotator` (`SceneComponent.RelativeRotation` NewParam)))
  (if (`self.CanTurn`)
    (set `self.CanTurn` false)
    (`KismetSystemLibrary.MoveComponentTo` NewParam (`SceneComponent.RelativeLocation` NewParam) (`KismetMathLibrary.MakeRotator` (+ _relativerotation_roll 60.0) _relativerotation_pitch _relativerotation_yaw))
    (set `self.CanTurn` true)
    (`self.CheckForWin`)))

(event `CheckForWin`
  (set `self.Points` 0)
  (`|ExecutionSequence`
    (:`then_0`
      (if (== (`SceneComponent.RelativeRotation` (`self.Sphere`)) (struct :`Roll` 180.0) :`ErrorTolerance` 30.0)
        (`/Engine/EditorBlueprintResources/StandardMacros.IncrementInt` (`self.Points`)
          (:`  `
            (`PrimitiveComponent.SetMaterial` (`self.Sphere`) 0 "/Engine/VREditor/UI/ArrowMaterial.ArrowMaterial")))
        (else
          (`PrimitiveComponent.SetMaterial` (`self.Sphere`) 0 "/Engine/BasicShapes/BasicShapeMaterial.BasicShapeMaterial"))))
    (:`then_1`
      (if (== (`SceneComponent.RelativeRotation` (`self.Sphere1`)) (struct :`Roll` -40.0) :`ErrorTolerance` 30.0)
        (`/Engine/EditorBlueprintResources/StandardMacros.IncrementInt` (`self.Points`)
          (:`  `
            (`PrimitiveComponent.SetMaterial` (`self.Sphere1`) 0 "/Engine/VREditor/UI/ArrowMaterial.ArrowMaterial")))
        (else
          (`PrimitiveComponent.SetMaterial` (`self.Sphere1`) 0 "/Engine/BasicShapes/BasicShapeMaterial.BasicShapeMaterial"))))
    (:`then_2`
      (if (== (`SceneComponent.RelativeRotation` (`self.Sphere2`)) (struct :`Roll` 30.0) :`ErrorTolerance` 30.0)
        (`/Engine/EditorBlueprintResources/StandardMacros.IncrementInt` (`self.Points`)
          (:`  `
            (`PrimitiveComponent.SetMaterial` (`self.Sphere2`) 0 "/Engine/VREditor/UI/ArrowMaterial.ArrowMaterial")))
        (else
          (`PrimitiveComponent.SetMaterial` (`self.Sphere2`) 0 "/Engine/BasicShapes/BasicShapeMaterial.BasicShapeMaterial"))))
    (:`then_3`
      (if (>= (`self.Points`) 3)
        (`PrimitiveComponent.SetMaterial` (`self.Sphere`) 0 "/Engine/MapTemplates/Materials/BasicAsset03.BasicAsset03")
        (`PrimitiveComponent.SetMaterial` (`self.Sphere1`) 0 "/Engine/MapTemplates/Materials/BasicAsset03.BasicAsset03")
        (`PrimitiveComponent.SetMaterial` (`self.Sphere2`) 0 "/Engine/MapTemplates/Materials/BasicAsset03.BasicAsset03")))))

(fn `UserConstructionScript`)