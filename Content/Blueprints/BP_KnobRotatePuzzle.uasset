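; Doorknob puzzle actor that opens the BP_PuzzleDooorONE door after the knob is turned three times.
; The Puzzleer event enables turning and slides Sphere, hidden at BeginPlay, when passed Doorknobnew.
; Any other input rolls Sphere1 a third of a turn via MoveComponentTo, with CanTurn blocking re-triggering mid-move.
; SpinNumber counts turns, then the actor calls OpenDoor on the door found at BeginPlay and destroys itself.
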(event `/Game/Blueprints/BPI_Puzzler.Puzzleer`
  (params (NewParam :type "SceneComponent Object Reference"))
  (bind _sphere1 (`self.Sphere1`))
  (bind (_relativerotation_roll _relativerotation_pitch _relativerotation_yaw) (`KismetMathLibrary.BreakRotator` (`SceneComponent.RelativeRotation` _sphere1)))
  (if (== NewParam (`self.Doorknobnew`))
    (set `self.CanTurn` true)
    (`KismetSystemLibrary.MoveComponentTo` (`self.Sphere`) (458.590186 2.222222 0.0) (struct) false false 1.0)
    (elif (`self.CanTurn`)
      (set `self.CanTurn` false)
      (`KismetSystemLibrary.MoveComponentTo` _sphere1 (-60.0 0.0 60.0) (`KismetMathLibrary.MakeRotator` (+ _relativerotation_roll 120.0) _relativerotation_pitch _relativerotation_yaw) false false 2.0)
      (bind _result (`/Engine/EditorBlueprintResources/StandardMacros.IncrementInt` (`self.SpinNumber`))
        (:`  `
          (set `self.CanTurn` true)
          (if (>= _result 3)
            (`/Game/Blueprints/BP_PuzzleDooorONE.OpenDoor` (`self.Door`))
            (`self.K2_DestroyActor`)))))))

(event `self.ReceiveBeginPlay`
  (`SceneComponent.SetVisibility` (`self.Sphere`) false true)
  (bind _returnvalue (`GameplayStatics.GetActorOfClass` "/Game/Blueprints/BP_PuzzleDooorONE.BP_PuzzleDooorONE_C"))
  (set `self.Door` _returnvalue))

(fn `UserConstructionScript`)