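; Door knob puzzle actor where a knob is turned repeatedly until it moves out of place and can be transferred to another puzzle.
; The Puzzleer event rolls the Sphere a half turn per call, gated by CanTurn, until a spin counter threshold sets Activate and slides it to a fixed relative pose.
; Once activated, the next call hides Sphere and Cube and reveals the Sphere on the first BP_KnobRotatePuzzle found in the level.
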(event `/Game/Blueprints/BPI_Puzzler.Puzzleer`
  (params (NewParam :type "SceneComponent Object Reference"))
  (bind _sphere (`self.Sphere`))
  (bind _returnvalue (`SceneComponent.GetRelativeTransform` _sphere))
  (if (== NewParam (`self.Sphere`))
    (if (`self.Activate`)
      (`SceneComponent.SetVisibility` (`self.Sphere`) false false)
      (`SceneComponent.SetVisibility` (`self.Cube`) false false)
      (bind _outactors (`GameplayStatics.GetAllActorsOfClass` "/Game/Blueprints/BP_KnobRotatePuzzle.BP_KnobRotatePuzzle_C"))
      (bind _sphere_2 (`/Game/Blueprints/BP_KnobRotatePuzzle.Sphere` (`|GetArrayItem` _outactors)))
      (`/Engine/EditorBlueprintResources/StandardMacros.IsValid` _sphere_2
        (:`Is Valid`
          (`SceneComponent.SetVisibility` _sphere_2 true true)))
      (elif (`self.CanTurn`)
        (set `self.CanTurn` false)
        (`KismetSystemLibrary.MoveComponentTo` _sphere (.location _returnvalue) (`KismetMathLibrary.MakeRotator` (+ (.roll (.rotation _returnvalue)) 180.0) (.pitch (.rotation _returnvalue)) (.yaw (.rotation _returnvalue))) false false 0.5)
        (bind _result (`/Engine/EditorBlueprintResources/StandardMacros.IncrementInt` (`self.SpinNumber`))
          (:`  `
            (set `self.CanTurn` true)
            (if (>= _result 4)
              (set `self.Activate` true)
              (`KismetSystemLibrary.MoveComponentTo` (`self.Sphere`) (60.0 0.0 -50.0) (struct :`Pitch` -90.0) true false 1.0))))))))

(fn `UserConstructionScript`)