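; Five-button sequence puzzle that flashes Button1 to Button5 green in a fixed order for the player to repeat.
; SimonSays replays the demo through delayed recursion until Puzzleer receives input, with CanActive gating overlap.
; Puzzleer passes presses after the first to Activator, which turns correct buttons gold and reveals connecting lines, including Line5 on completion.
; Out-of-order presses through Activator hide the lines, flash all buttons red, reset progress and restart the demo.
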(event `Activator`
  (params (ReqPoints :type Integer) (Button :type "StaticMeshComponent Object Reference") (Line :type "StaticMeshComponent Object Reference"))
  (if (== (`self.Points`) ReqPoints)
    (`PrimitiveComponent.SetMaterial` Button 0 "/Game/Blueprints/Assets/GOLD.GOLD")
    (`SceneComponent.SetVisibility` Line true false)
    (`/Engine/EditorBlueprintResources/StandardMacros.IncrementInt` (`self.Points`)
      (:`  `
        (set `self.CanActive` true)))
    (else
      (for _array_element (`self.Lines`)
        (`SceneComponent.SetVisibility` _array_element false false))
      (`self.Wrong`))))

(event `Wrong`
  (for _array_element (`self.Buttons`)
    (`PrimitiveComponent.SetMaterial` _array_element 0 "/Game/Blueprints/Assets/RED.RED"))
  (`KismetSystemLibrary.Delay` 1.0)
  (for _array_element_2 (`self.Buttons`)
    (`PrimitiveComponent.SetMaterial` _array_element_2 0 "/Engine/BasicShapes/BasicShapeMaterial.BasicShapeMaterial"))
  (set `self.CanActive` true)
  (set `self.Points` 0)
  (set `self.OnGame` false)
  (`self.SimonSays`))

(event `self.ReceiveBeginPlay`
  (`self.SimonSays`)
  (set `self.Buttons` (`|MakeArray` (`self.Button 1`) (`self.Button 2`) (`self.Button 3`) (`self.Button 4`) (`self.Button 5`)))
  (set `self.Lines` (`|MakeArray` (`self.Line 1`) (`self.Line 2`) (`self.Line 3`) (`self.Line 4`) (`self.Line 5`))))

(event `SimonSays`
  (if (`self.OnGame`)
    _
    (elif (`self.CanActive`)
      (set `self.CanActive` false)
      (`PrimitiveComponent.SetMaterial` (`self.Button 1`) 0 "/Game/Blueprints/Assets/GREEN.GREEN")
      (`KismetSystemLibrary.Delay` 0.7)
      (`PrimitiveComponent.SetMaterial` (`self.Button 1`) 0 "/Engine/BasicShapes/BasicShapeMaterial.BasicShapeMaterial")
      (`PrimitiveComponent.SetMaterial` (`self.Button 2`) 0 "/Game/Blueprints/Assets/GREEN.GREEN")
      (`KismetSystemLibrary.Delay` 0.7)
      (`PrimitiveComponent.SetMaterial` (`self.Button 2`) 0 "/Engine/BasicShapes/BasicShapeMaterial.BasicShapeMaterial")
      (`PrimitiveComponent.SetMaterial` (`self.Button 3`) 0 "/Game/Blueprints/Assets/GREEN.GREEN")
      (`KismetSystemLibrary.Delay` 0.7)
      (`PrimitiveComponent.SetMaterial` (`self.Button 3`) 0 "/Engine/BasicShapes/BasicShapeMaterial.BasicShapeMaterial")
      (`PrimitiveComponent.SetMaterial` (`self.Button 4`) 0 "/Game/Blueprints/Assets/GREEN.GREEN")
      (`KismetSystemLibrary.Delay` 0.7)
      (`PrimitiveComponent.SetMaterial` (`self.Button 4`) 0 "/Engine/BasicShapes/BasicShapeMaterial.BasicShapeMaterial")
      (`PrimitiveComponent.SetMaterial` (`self.Button 5`) 0 "/Game/Blueprints/Assets/GREEN.GREEN")
      (`KismetSystemLibrary.Delay` 0.7)
      (`PrimitiveComponent.SetMaterial` (`self.Button 5`) 0 "/Engine/BasicShapes/BasicShapeMaterial.BasicShapeMaterial")
      (set `self.CanActive` true)
      (`KismetSystemLibrary.Delay` 3.0)
      (`self.SimonSays`))))

(event `/Game/Blueprints/BPI_Puzzler.Puzzleer`
  (params (NewParam :type "SceneComponent Object Reference"))
  (if (`self.CanActive`)
    (set `self.CanActive` false)
    (set `self.OnGame` true)
    (if (== NewParam (`self.Button 1`))
      (if (== (`self.Points`) 0)
        (`PrimitiveComponent.SetMaterial` (`self.Button 1`) 0 "/Game/Blueprints/Assets/GOLD.GOLD")
        (`/Engine/EditorBlueprintResources/StandardMacros.IncrementInt` (`self.Points`)
          (:`  `
            (set `self.CanActive` true))))
      (elif (== NewParam (`self.Button 2`))
        (`self.Activator` 1 (`self.Button 2`) (`self.Line 1`))
        (elif (== NewParam (`self.Button 3`))
          (`self.Activator` 2 (`self.Button 3`) (`self.Line 2`))
          (elif (== NewParam (`self.Button 4`))
            (`self.Activator` 3 (`self.Button 4`) (`self.Line 3`))
            (elif (== NewParam (`self.Button 5`))
              (`self.Activator` 4 (`self.Button 5`) (`self.Line 4`))
              (if (>= (`self.Points`) 5)
                (`SceneComponent.SetVisibility` (`self.Line 5`) true false))
              (elif (or (== NewParam (`self.Button 1`)) (== NewParam (`self.Button 2`)) (== NewParam (`self.Button 3`)) (== NewParam (`self.Button 4`)) (== NewParam (`self.Button 5`)))
                (`self.Wrong`)
                (else
                  (if (== (`self.Points`) 0)
                    (set `self.OnGame` false))
                  (set `self.CanActive` true))))))))))

(fn `UserConstructionScript`)