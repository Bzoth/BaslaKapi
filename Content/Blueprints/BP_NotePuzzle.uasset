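; BP_NotePuzzle is a musical button puzzle that opens BP_PuzzleDooorONE when notes are pressed in the order La, Mi, Re, Si.
; Puzzleer plays a sound for the pressed note, then CheckForNote uses a Points counter to validate order and turn correct buttons green.
; A mistake resets Points, flashes WrongLight and restores only the Do, Mi, La and Fa materials.
; Success lights RightLight, opens the door and destroys the puzzle actor.
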(event `Wrong`
  (bind _wronglight (`self.WrongLight`))
  (`PrimitiveComponent.SetMaterial` _wronglight 0 "/Game/Blueprints/Assets/REDLIGHT.REDLIGHT")
  (`KismetSystemLibrary.Delay` 1.0)
  (`PrimitiveComponent.SetMaterial` _wronglight 0 "/Game/Blueprints/Assets/RED.RED")
  (for _array_element (`self.Buttons`)
    (`PrimitiveComponent.SetMaterial` _array_element 0 "/Engine/BasicShapes/BasicShapeMaterial.BasicShapeMaterial")))

(event `self.ReceiveBeginPlay`
  (set `self.Buttons` (`|MakeArray` (`self.Do`) (`self.Mi`) (`self.La`) (`self.Fa`)))
  (bind _returnvalue (`GameplayStatics.GetActorOfClass` "/Game/Blueprints/BP_PuzzleDooorONE.BP_PuzzleDooorONE_C"))
  (set `self.Door` _returnvalue))

(event `/Game/Blueprints/BPI_Puzzler.Puzzleer`
  (params (NewParam :type "SceneComponent Object Reference"))
  (bind _re (`self.Re`))
  (bind _la (`self.La`))
  (bind _mi (`self.Mi`))
  (bind _si (`self.Si`))
  (`|ExecutionSequence`
    (:`then_0`
      (`|ExecutionSequence`
        (:`then_0`
          (if (== NewParam (`self.Do`))
            (`GameplayStatics.PlaySound2D` null 1.0 1.0 0.0 null null)))
        (:`then_1`
          (if (== NewParam (`self.Re`))
            (`GameplayStatics.PlaySound2D` null 1.0 1.0 0.0 null null)))
        (:`then_2`
          (if (== NewParam (`self.Mi`))
            (`GameplayStatics.PlaySound2D` null 1.0 1.0 0.0 null null)))
        (:`then_3`
          (if (== NewParam (`self.Fa`))
            (`GameplayStatics.PlaySound2D` null 1.0 1.0 0.0 null null)))
        (:`then_4`
          (if (== NewParam (`self.Sol`))
            (`GameplayStatics.PlaySound2D` null 1.0 1.0 0.0 null null)))
        (:`then_5`
          (if (== NewParam (`self.La`))
            (`GameplayStatics.PlaySound2D` null 1.0 1.0 0.0 null null)))
        (:`then_6`
          (if (== NewParam (`self.Si`))
            (`GameplayStatics.PlaySound2D` null 1.0 1.0 0.0 null null)))))
    (:`then_1`
      (if (== NewParam _la)
        (`self.CheckForNote` 0 _la)
        (elif (== NewParam _mi)
          (`self.CheckForNote` 1 _mi)
          (elif (== NewParam _re)
            (`self.CheckForNote` 2 _re)
            (elif (== NewParam _si)
              (`self.CheckForNote` 3 _si)
              (if (>= (`self.Points`) 4)
                (`PrimitiveComponent.SetMaterial` (`self.RightLight`) 0 "/Game/Blueprints/Assets/GREENLIGHT.GREENLIGHT")
                (`/Game/Blueprints/BP_PuzzleDooorONE.OpenDoor` (`self.Door`))
                (`self.K2_DestroyActor`))
              (else
                (set `self.Points` 0)
                (`self.Wrong`)))))))))

(fn `CheckForNote`
  (params (ReqPoints :type Integer) (Note :type "PrimitiveComponent Object Reference"))
  (if (== (`self.Points`) ReqPoints)
    (`/Engine/EditorBlueprintResources/StandardMacros.IncrementInt` (`self.Points`)
      (:`  `
        (`PrimitiveComponent.SetMaterial` Note 0 "/Game/Blueprints/Assets/GREEN.GREEN")))
    (else
      (set `self.Points` 0)
      (`self.Wrong`))))

(fn `UserConstructionScript`)