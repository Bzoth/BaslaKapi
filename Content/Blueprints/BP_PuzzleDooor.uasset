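; BP_PuzzleDooor is a puzzle door that swings open once its OpenDoor event has been called at least three times.
; Each OpenDoor call increments a Point counter, and reaching the threshold rotates the Scene component open with MoveComponentTo.
; Any actor beginning overlap with the Box component triggers CloseDoor, which rotates the door back to zero without resetting the counter.
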(event `self.Box.OnComponentBeginOverlap`
  (params (OverlappedComponent :type "PrimitiveComponent Object Reference") (OtherActor :type "Actor Object Reference") (OtherComp :type "PrimitiveComponent Object Reference") (OtherBodyIndex :type Integer) (bFromSweep :type Boolean) (SweepResult :type "HitResult Structure (by ref)"))
  (`self.CloseDoor`))

(event `OpenDoor`
  (bind _result (`/Engine/EditorBlueprintResources/StandardMacros.IncrementInt` (`self.Point`))
    (:`  `
      (if (>= _result 3)
        (`KismetSystemLibrary.MoveComponentTo` (`self.Scene`) (0.0 0.0 0.0) (struct :`Yaw` -100.0))))))

(event `CloseDoor`
  (`KismetSystemLibrary.MoveComponentTo` (`self.Scene`) (0.0 0.0 0.0) (struct)))

(fn `UserConstructionScript`)