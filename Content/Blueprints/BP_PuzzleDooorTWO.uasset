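; BP_PuzzleDooorTWO is a puzzle door that swings open once its point count reaches a threshold.
; It caches the first-person character on BeginPlay.
; OpenDoor restores the player camera and increments the counter, then rotates the Scene component with MoveComponentTo and destroys the linked puzzle actors when the threshold is met.
; CloseDoor moves the same component back to default relative transform values.
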(event `self.ReceiveBeginPlay`
  (bind _asbp_first_person_character (cast `/Game/FirstPerson/Blueprints/BP_FirstPersonCharacter` (`GameplayStatics.GetPlayerCharacter` 0)))
  (set `self.Player` _asbp_first_person_character))

(event `OpenDoor`
  (`/Game/FirstPerson/Blueprints/BP_FirstPersonCharacter.ReturnPlayerCam` (`self.Player`))
  (bind _result (`/Engine/EditorBlueprintResources/StandardMacros.IncrementInt` (`self.Point`))
    (:`  `
      (if (>= _result 1)
        (`KismetSystemLibrary.MoveComponentTo` (`self.Scene`) (0.0 0.0 0.0) (struct :`Yaw` -190.0) false false 1.0)
        (for _array_element (`self.Puzzless`)
          (`self.K2_DestroyActor` _array_element))))))

(event `CloseDoor`
  (`KismetSystemLibrary.MoveComponentTo` (`self.Scene`)))

(fn `UserConstructionScript`)